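; Player-controlled hover vehicle, driven by physics impulses on its body and set up with four corner hover components.
; Movement input adds mass-scaled thrust below a speed threshold, while turning rotates the body and applies a velocity-correcting impulse.
; Each tick, holding Left Shift adds boost thrust, enables trail effects and shortens the camera spring arm.
; The spring arm also tilts with steep body pitch and eases back toward its initial angle.
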(event `InputAxis|MoveForward/BackWard`
  (params (AxisValue :type "Float (single-precision)"))
  (bind _player (`self.Player`))
  (bind (_returnvalue_roll _returnvalue_pitch) (`KismetMathLibrary.BreakRotator` (`SceneComponent.K2_GetComponentRotation` _player)))
  (bind (_returnvalue_roll_2 _returnvalue_pitch_2) (`KismetMathLibrary.BreakRotator` (`SceneComponent.K2_GetComponentRotation` (`self.Camera`))))
  (bind (_returnvalue_x _returnvalue_y) (`KismetMathLibrary.BreakVector` (`SceneComponent.GetComponentVelocity` (`self.Player`))))
  ;[1 1 1] Mouvement Velocity
  (`/Engine/EditorBlueprintResources/StandardMacros.CompareFloat` (+ (`KismetMathLibrary.Abs` _returnvalue_x) (`KismetMathLibrary.Abs` _returnvalue_y)) 10000.0
    (:`<`
      (`PrimitiveComponent.AddImpulse` _player (* (* (`SceneComponent.GetForwardVector` (`self.Player`)) -1.0) (* AxisValue (`PrimitiveComponent.GetMass` (`self.Player`)) 500.0)) "None" false)
      (if (< _returnvalue_pitch -5.0)
        (if (< _returnvalue_pitch_2 10.0)
          _)))))

(event `InputAxis|TurnRight/Left`
  (params (AxisValue :type "Float (single-precision)"))
  (bind _returnvalue (`SceneComponent.GetComponentVelocity` (`self.Player`)))
  ;[1 1 1] Turn Left Right
  (`SceneComponent.K2_AddLocalRotation` (`self.Player`) (`KismetMathLibrary.MakeRotator` 0.0 0.0 (* AxisValue 2.0)) false false)
  (`PrimitiveComponent.AddImpulse` (`self.Player`) (- (* _returnvalue (`SceneComponent.GetForwardVector` (`self.Player`))) _returnvalue) "None" false))

(event `self.ReceiveTick`
  (params (DeltaSeconds :type "Float (single-precision)"))
  (bind _player (`self.Player`))
  (bind _targetarmlength (`SpringArmComponent.TargetArmLength` (`self.SpringArm`)))
  (bind _returnvalue (- _targetarmlength 10.0))
  (bind _returnvalue_2 (+ _targetarmlength 10.0))
  ;[1 1 1] Boost
  (bind _output_get (set `self.isBoosting` (`PlayerController.IsInputKeyDown` (`GameplayStatics.GetPlayerController` 0) "LeftShift")))
  (if _output_get
    (`PrimitiveComponent.AddImpulse` (`self.Player`) (* (`SceneComponent.GetForwardVector` _player) (* -750.0 (`PrimitiveComponent.GetMass` _player))) "None" false))
  (`ActorComponent.SetActive` (`self.TrailRight2`) (`self.isBoosting`) false)
  (`ActorComponent.SetActive` (`self.TrailLeft2`) (`self.isBoosting`) false)
  (`FXSystemComponent.SetEmitterEnable` (`self.TrailLeft1`) "MotorLightBoost" (`self.isBoosting`))
  (`FXSystemComponent.SetEmitterEnable` (`self.TrailRight1`) "MotorLightBoost" (`self.isBoosting`))
  (`FXSystemComponent.SetEmitterEnable` (`self.TrailRight2`) "MotorLightBoost" (`self.isBoosting`))
  (`FXSystemComponent.SetEmitterEnable` (`self.TrailLeft2`) "MotorLightBoost" (`self.isBoosting`))
  (`FXSystemComponent.SetEmitterEnable` (`self.MainTrail`) "MainTailBoost" (`self.isBoosting`))
  ;;[1 1 1] CameraManagement
  (if (`self.isBoosting`)
    (if (> _returnvalue 600.0)
      (set `SpringArmComponent.TargetArmLength` _returnvalue (`self.SpringArm`)))
    (elif (< _returnvalue_2 1000.0)
      (bind _output_get_2 (set `SpringArmComponent.TargetArmLength` _returnvalue_2 (`self.SpringArm`)))))
  (`self.ManageCamera`))

(event `self.ReceiveBeginPlay`
  ;[1 1 1] Init
  (`self.InitHovers`)
  (`FXSystemComponent.SetEmitterEnable` (`self.TrailLeft1`) "MotorLightBoost" false)
  (`FXSystemComponent.SetEmitterEnable` (`self.TrailRight1`) "MotorLightBoost" false)
  (`FXSystemComponent.SetEmitterEnable` (`self.MainTrail`) "MainTailBoost" false)
  (set `self.IntialCameraRotation` (`SceneComponent.RelativeRotation` (`self.SpringArm`))))

(fn `InitHovers`
  (bind _player (`self.Player`))
  (`/Game/Blueprints/HoverComponont.InitHover` (`self.HoverComponontBL`) _player)
  (`/Game/Blueprints/HoverComponont.InitHover` (`self.HoverComponontBR`) _player)
  (`/Game/Blueprints/HoverComponont.InitHover` (`self.HoverComponontFL`) _player)
  (`/Game/Blueprints/HoverComponont.InitHover` (`self.HoverComponontFR`) _player))

(fn `ManageCamera`
  (bind _springarm (`self.SpringArm`))
  (bind (_intialcamerarotation_roll _intialcamerarotation_pitch) (`KismetMathLibrary.BreakRotator` (`self.IntialCameraRotation`)))
  (bind (_intialcamerarotation_roll_2 _intialcamerarotation_pitch_2) (`KismetMathLibrary.BreakRotator` (`self.IntialCameraRotation`)))
  (bind _springarm_2 (`self.SpringArm`))
  (bind (_returnvalue_roll _returnvalue_pitch) (`KismetMathLibrary.BreakRotator` (`SceneComponent.K2_GetComponentRotation` (`self.Player`))))
  (bind (_returnvalue_roll_2 _returnvalue_pitch_2) (`KismetMathLibrary.BreakRotator` (`SceneComponent.K2_GetComponentRotation` _springarm)))
  (bind (_returnvalue_roll_3 _returnvalue_pitch_3) (`KismetMathLibrary.BreakRotator` (`SceneComponent.K2_GetComponentRotation` _springarm_2)))
  (bind (_relativerotation_roll _relativerotation_pitch) (`KismetMathLibrary.BreakRotator` (`SceneComponent.RelativeRotation` (`self.SpringArm`))))
  (bind (_relativerotation_roll_2 _relativerotation_pitch_2) (`KismetMathLibrary.BreakRotator` (`SceneComponent.RelativeRotation` (`self.SpringArm`))))
  (if (< _returnvalue_pitch -10.0)
    (if (< _returnvalue_pitch_3 30.0)
      (`SceneComponent.K2_AddRelativeRotation` _springarm_2 (`KismetMathLibrary.MakeRotator` 0.0 0.5) true false))
    (elif (> _returnvalue_pitch 10.0)
      (if (> _returnvalue_pitch_2 -40.0)
        (`SceneComponent.K2_AddRelativeRotation` _springarm (`KismetMathLibrary.MakeRotator` 0.0 -0.5) true false))
      (elif (< _relativerotation_pitch_2 (- _intialcamerarotation_pitch_2 1.0))
        (`SceneComponent.K2_AddRelativeRotation` (`self.SpringArm`) (`KismetMathLibrary.MakeRotator` 0.0 1.0) true false)
        (elif (> _relativerotation_pitch (+ _intialcamerarotation_pitch 1.0))
          (`SceneComponent.K2_AddRelativeRotation` (`self.SpringArm`) (`KismetMathLibrary.MakeRotator` 0.0 -1.0) true false))))))

(fn `UserConstructionScript`)