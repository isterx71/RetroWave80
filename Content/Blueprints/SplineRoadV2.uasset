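; Spline road actor that builds a road out of spline mesh segments in its construction script.
; It resizes the RoadDatas array to the spline point count, though the mesh build never reads that array.
; Segments follow the spline by distance at SpaceBetween intervals, using world-space positions and scaled directions as tangents.
; Each gets the road mesh, material, uniform roll and width, plus optional blocking collision.
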(fn `UserConstructionScript`
  (locals (LocalSplineMesh :type "SplineMeshComponent Object Reference") (LocalCurrentIndex :type Integer) (`Local Next Index` :type Integer :default 0) (LocalLocationCurrentPoint :type "Vector Structure" :default (0.0 0.0 0.0)) (LocalTangenteCurrentPoint :type "Vector Structure" :default (0.0 0.0 0.0)) (LocalLocationNextPoint :type "Vector Structure" :default (0.0 0.0 0.0)) (LocalTangenteNextPoint :type "Vector Structure" :default (0.0 0.0 0.0)))
  (bind _roaddatas (`self.RoadDatas`))
  (bind _rooling (`self.Rooling`))
  (bind _spacebetween (`self.SpaceBetween`))
  (bind _localsplinemesh (`local.LocalSplineMesh`))
  (bind _localsplinemesh_2 (`local.LocalSplineMesh`))
  (bind _localsplinemesh_3 (`local.LocalSplineMesh`))
  (bind _largest (`self.Largest`))
  (bind _spline (`self.Spline`))
  (bind _tangent (`self.Tangent`))
  (bind (_remainder _returnvalue) (`KismetMathLibrary.FMod` (`SplineComponent.GetSplineLength` (`self.Spline`)) _spacebetween))
  (`|ExecutionSequence`
    (:`then_0`
      (set `self.NbSplinePoint` (`SplineComponent.GetNumberOfSplinePoints` (`self.Spline`))))
    (:`then_1`
      (`/Engine/EditorBlueprintResources/StandardMacros.CompareInt` (`KismetArrayLibrary.Array_Length` (`self.RoadDatas`)) (`self.NbSplinePoint`) :!label _label
        (:`>`
          (`KismetArrayLibrary.Array_Remove` _roaddatas (`KismetArrayLibrary.Array_LastIndex` _roaddatas))
          (goto _label))
        (:`<`
          (`KismetArrayLibrary.Array_Add` (`self.RoadDatas`))
          (goto _label))))
    (:`then_2`
      (for _index (range (+ _returnvalue 1))
        (bind _output_get (set `local.LocalCurrentIndex` _index))
        (set `local.Local Next Index` (mod (+ _output_get 1) _returnvalue))
        (bind _returnvalue_2 (`AddComponent|NODE_AddSplineMeshComponent-1` :`bManualAttachment` true))
        (set `local.LocalSplineMesh` _returnvalue_2)
        (`StaticMeshComponent.SetStaticMesh` (`local.LocalSplineMesh`) (`self.road`))
        (`PrimitiveComponent.SetMaterial` (`local.LocalSplineMesh`) 0 (`self.material`))
        (bind _returnvalue_3 (* _index _spacebetween))
        (bind _returnvalue_4 (+ _returnvalue_3 _spacebetween))
        (`SplineMeshComponent.SetStartAndEnd` (`local.LocalSplineMesh`) (`SplineComponent.GetLocationAtDistanceAlongSpline` _spline _returnvalue_3 "World") (* (`SplineComponent.GetDirectionAtDistanceAlongSpline` _spline _returnvalue_3 "World") _tangent) (`SplineComponent.GetLocationAtDistanceAlongSpline` _spline _returnvalue_4 "World") (* (`SplineComponent.GetDirectionAtDistanceAlongSpline` _spline _returnvalue_4 "World") _tangent) true)
        (`|ExecutionSequence`
          (:`then_0`
            (if (`self.Collision`)
              (`PrimitiveComponent.SetCollisionEnabled` _localsplinemesh_2 "QueryAndPhysics")
              (`PrimitiveComponent.SetCollisionResponseToAllChannels` _localsplinemesh_2 "ECR_Block")))
          (:`then_1`
            (`SplineMeshComponent.SetStartRoll` _localsplinemesh_3 _rooling true)
            (`SplineMeshComponent.SetEndRoll` _localsplinemesh_3 _rooling true))
          (:`then_2`
            (`SplineMeshComponent.SetStartScale` _localsplinemesh (`KismetMathLibrary.MakeVector2D` _largest 1.0) true)
            (`SplineMeshComponent.SetEndScale` _localsplinemesh (`KismetMathLibrary.MakeVector2D` _largest 1.0) true)))))))