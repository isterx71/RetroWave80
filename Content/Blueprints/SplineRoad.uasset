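; Spline road Blueprint that builds a deformed road mesh along an editable spline in its construction script.
; It resizes the RoadDatas array to match the point count, then adds one spline mesh per segment, using per-point roll and width at each end.
; Toggles enable blocking collision and point-index text labels, which are re-created on every segment iteration.
; Unconnected leftover nodes sketch an alternative fixed-spacing placement by distance.
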(fn `UserConstructionScript`
  (locals (LocalSplineMesh :type "SplineMeshComponent Object Reference") (LocalCurrentIndex :type Integer) (`Local Next Index` :type Integer :default 0) (LocalLocationCurrentPoint :type "Vector Structure" :default (0.0 0.0 0.0)) (LocalTangenteCurrentPoint :type "Vector Structure" :default (0.0 0.0 0.0)) (LocalLocationNextPoint :type "Vector Structure" :default (0.0 0.0 0.0)) (LocalTangenteNextPoint :type "Vector Structure" :default (0.0 0.0 0.0)) (LocalSplinePointText :type Text))
  (bind _roaddatas (`self.RoadDatas`))
  (bind _localsplinemesh (`local.LocalSplineMesh`))
  (bind _localsplinemesh_2 (`local.LocalSplineMesh`))
  (bind _localsplinemesh_3 (`local.LocalSplineMesh`))
  (bind (_location _tangent) (`SplineComponent.GetLocationAndTangentAtSplinePoint` (`self.Spline`) (`local.Local Next Index`) "World"))
  (bind (_location_2 _tangent_2) (`SplineComponent.GetLocationAndTangentAtSplinePoint` (`self.Spline`) (`local.LocalCurrentIndex`) "World"))
  (bind (_output_roadwith _output_roadroll) (break `/Game/Data/RoadDatas` (`|GetArrayItem` (`self.RoadDatas`) (`local.Local Next Index`))))
  (bind (_output_roadwith_2 _output_roadroll_2) (break `/Game/Data/RoadDatas` (`|GetArrayItem` (`self.RoadDatas`) (`local.LocalCurrentIndex`))))
  (bind _output_roadwith_3 (break `/Game/Data/RoadDatas` (`|GetArrayItem` (`self.RoadDatas`) (`local.Local Next Index`))))
  (bind _output_roadwith_4 (break `/Game/Data/RoadDatas` (`|GetArrayItem` (`self.RoadDatas`) (`local.LocalCurrentIndex`))))
  (`|ExecutionSequence`
    (:`then_0`
      (set `self.NbSplinePoint` (`SplineComponent.GetNumberOfSplinePoints` (`self.Spline`))))
    (:`then_1`
      (`/Engine/EditorBlueprintResources/StandardMacros.CompareInt` (`KismetArrayLibrary.Array_Length` (`self.RoadDatas`)) (`self.NbSplinePoint`) :!label _label
        (:`>`
          (`KismetArrayLibrary.Array_Remove` _roaddatas (`KismetArrayLibrary.Array_LastIndex` _roaddatas))
          (goto _label))
        (:`<`
          (`KismetArrayLibrary.Array_Add` (`self.RoadDatas`))
          (goto _label))))
    (:`then_2`
      (for _index (range (+ (- (`self.NbSplinePoint`) 2) 1))
        (`|ExecutionSequence`
          (:`then_0`
            (bind _output_get (set `local.LocalCurrentIndex` _index))
            (set `local.Local Next Index` (mod (+ _output_get 1) (`self.NbSplinePoint`))))
          (:`then_1`
            (set `local.LocalLocationCurrentPoint` _location_2)
            (set `local.LocalTangenteCurrentPoint` _tangent_2)
            (set `local.LocalLocationNextPoint` _location)
            (set `local.LocalTangenteNextPoint` _tangent))
          (:`then_2`
            (bind _returnvalue (`AddComponent|NODE_AddSplineMeshComponent-1` :`bManualAttachment` true))
            (set `local.LocalSplineMesh` _returnvalue)
            (`StaticMeshComponent.SetStaticMesh` (`local.LocalSplineMesh`) (`self.road`))
            (`PrimitiveComponent.SetMaterial` (`local.LocalSplineMesh`) 0 (`self.material`))
            (`SplineMeshComponent.SetStartAndEnd` (`local.LocalSplineMesh`) (`local.LocalLocationCurrentPoint`) (`local.LocalTangenteCurrentPoint`) (`local.LocalLocationNextPoint`) (`local.LocalTangenteNextPoint`) true)
            (`|ExecutionSequence`
              (:`then_0`
                (if (`self.Collision`)
                  (`PrimitiveComponent.SetCollisionEnabled` _localsplinemesh_2 "QueryAndPhysics")
                  (`PrimitiveComponent.SetCollisionResponseToAllChannels` _localsplinemesh_2 "ECR_Block")))
              (:`then_1`
                (`SplineMeshComponent.SetStartRoll` _localsplinemesh_3 _output_roadroll_2 true)
                (`SplineMeshComponent.SetEndRoll` _localsplinemesh_3 _output_roadroll true))
              (:`then_2`
                (`SplineMeshComponent.SetStartScale` _localsplinemesh (`KismetMathLibrary.MakeVector2D` _output_roadwith_4 1.0) true)
                (`SplineMeshComponent.SetEndScale` _localsplinemesh (`KismetMathLibrary.MakeVector2D` _output_roadwith_3 1.0) true))
              (:`then_3`
                (if (`self.showPointSpline`)
                  (for _index_2 (range (`self.NbSplinePoint`))
                    (set `local.LocalSplinePointText` (`KismetTextLibrary.Conv_IntToText` _index_2))
                    (bind (_location_3 _tangent_3) (`SplineComponent.GetLocationAndTangentAtSplinePoint` (`self.Spline`) _index_2 "Local"))
                    (bind _returnvalue_2 (`AddComponent|NODE_AddTextRenderComponent-0` :`RelativeTransform` (`KismetMathLibrary.MakeTransform` (`KismetMathLibrary.MakeVector` (.x _location_3) (.y _location_3) (+ (.z _location_3) 50.0)) (`KismetMathLibrary.Conv_VectorToRotator` (* _tangent_3 -1.0)))))
                    (`TextRenderComponent.K2_SetText` _returnvalue_2 (`local.LocalSplinePointText`))))))))))))