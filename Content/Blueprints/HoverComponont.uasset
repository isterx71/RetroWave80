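; Hover component that pushes a physics-simulated mesh, supplied through InitHover, away from surfaces below it.
; Each tick it line traces on Visibility, with the end point multiplying world location by the scaled down vector rather than adding it.
; A hit applies force along the impact normal at the component's location, fading from HoverForce with distance over LenghtTrace.
; Hits also set high linear and angular damping, which is never reset.
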(event `InitHover`
  (params (MeshComponent :type "StaticMeshComponent Object Reference"))
  (bind _output_get (set `self.Primitive Component` MeshComponent))
  (`PrimitiveComponent.SetSimulatePhysics` _output_get true))

(event `self.ReceiveTick`
  (params (DeltaSeconds :type "Float (single-precision)"))
  (bind _returnvalue (`self.K2_GetComponentLocation`))
  (bind _primitive_component (`self.Primitive Component`))
  (bind (_outhit _returnvalue_2) (`KismetSystemLibrary.LineTraceSingle` _returnvalue (* _returnvalue (* (`self.GetUp`) (* (`self.LenghtTrace`) -1.0))) "TraceTypeQuery1"))
  (if _returnvalue_2
    (bind (_bblockinghit _binitialoverlap _time _distance _location _impactpoint _normal _impactnormal) (`GameplayStatics.BreakHitResult` _outhit))
    (`PrimitiveComponent.AddForceAtLocation` _primitive_component (* _impactnormal (`KismetMathLibrary.Lerp` (`self.HoverForce`) 0.0 (/ (`KismetMathLibrary.VSize` (- _location (`self.K2_GetComponentLocation`))) (`self.LenghtTrace`)))) (`self.K2_GetComponentLocation`) "None")
    (`PrimitiveComponent.SetLinearDamping` _primitive_component 10.0)
    (`PrimitiveComponent.SetAngularDamping` _primitive_component 10.0)))